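; Game mode that displays the player HUD, tracks score, and flags when every light in the level has been passed.
; BeginPlay creates the PlayerUI widget and adds it to the viewport.
; Tick re-queries all BP_light actors every frame and sets Exploding once their count equals PassedLights, which this file never updates.
; AddScore increments TotalScore by one.
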(event `self.ReceiveBeginPlay`
  (bind _returnvalue (`|CreateWidget` "/Game/UMG/PlayerUI.PlayerUI_C"))
  (`UserWidget.AddToViewport` _returnvalue 0))

(event `self.ReceiveTick`
  (params (DeltaSeconds :type "Float (single-precision)"))
  (bind _outactors (`GameplayStatics.GetAllActorsOfClass` "/Game/Blueprints/BP_light.BP_light_C"))
  (bind _output_get (set `self.NumberOfLights` (`KismetArrayLibrary.Array_Length` _outactors)))
  (if (== _output_get (`self.PassedLights`))
    (set `self.Exploding` true)))

(fn `AddScore`
  (set `self.TotalScore` (+ (`self.TotalScore`) 1)))

(fn `UserConstructionScript`)